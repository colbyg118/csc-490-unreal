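; BP_NPC is an NPC Blueprint that opens a question-based dialogue UI when its Talk event is called.
; Talk lazily creates a WB_Dialogue widget for the first local player, caches it and sets its opening prompt on every call.
; It also creates and caches an Input widget, passing it the dialogue widget through a SetUIVariable interface message when first created.
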(event `/Game/Dialogue/BPI_Dialogue.Talk`
  (`self.UI`
    (:`then`
      _)
    (:`else`
      (bind _returnvalue (`|CreateWidget` "/Game/Dialogue/WB_Dialogue.WB_Dialogue_C" (`GameplayStatics.GetPlayerController` 0)))
      (bind _output_get (set `self.UI` _returnvalue))
      (`UserWidget.AddToViewport` _output_get 0)))
  (`TextBlock.SetText` (`/Game/Dialogue/WB_Dialogue.TalkText` (`self.UI`)) "Ask a me a question")
  (`self.InputUI`
    (:`then`)
    (:`else`
      (bind _returnvalue_2 (`|CreateWidget` "/Game/Dialogue/Input.Input_C" (`GameplayStatics.GetPlayerController` 0)))
      (bind _output_get_2 (set `self.InputUI` _returnvalue_2))
      (`UserWidget.AddToViewport` _output_get_2 0)
      (message `/Game/Dialogue/BPI_UI.SetUIVariable` (`self.InputUI`) (`self.UI`)))))

(fn `UserConstructionScript`)